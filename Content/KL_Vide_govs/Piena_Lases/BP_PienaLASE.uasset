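; Milk drip actor for a cow exhibit that animates falling drops and a filling milk level while an actor overlaps it.
; Overlap start loops the drop animation and runs a timeline that drives the milk level mesh's "PiensPilns" (milk full) morph target.
; Each timeline finish triggers a one-shot play call on the level mesh and restarts the fill.
; Overlap end stops and rewinds the drop animation and halts the timeline, without resetting the morph.
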(event `self.ReceiveBeginPlay`)

(event `self.ReceiveActorBeginOverlap`
  (params (OtherActor :type "Actor Object Reference"))
  (`SkeletalMeshComponent.PlayAnimation` (`self.SkeletalMeshComponent`) "/Game/KL_Vide_govs/Piena_Lases/govs_LASE_Anim01_Anim_LASE_viena_01_Cube_001Action.govs_LASE_Anim01_Anim_LASE_viena_01_Cube_001Action" true)
  (bind (_direction _newtrack_0) (`Timeline|Timeline` :!label _label)
    (:`Update`
      (`SkeletalMeshComponent.SetMorphTarget` (`self.govs_pienalimenis_01`) "PiensPilns" _newtrack_0 true))
    (:`Finished`
      (`SkeletalMeshComponent.PlayAnimation` (`self.govs_pienalimenis_01`) null false)
      (goto _label :!via `PlayFromStart`))))

(event `self.ReceiveActorEndOverlap`
  (params (OtherActor :type "Actor Object Reference"))
  (`SkeletalMeshComponent.Stop` (`self.SkeletalMeshComponent`))
  (`SkeletalMeshComponent.SetPosition` (`self.SkeletalMeshComponent`) 0.0 true)
  (goto _label :!via `Stop`))

(fn `UserConstructionScript`)